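; BP_Orco is an orc that moves steadily and periodically shoots arrows at a target archer.
; Tick applies VectorOrco as a local offset every frame, unscaled by delta time; SetPosicionOrco sets that vector using a speed multiplier.
; A looping timer calls Disparar, which, while PuedeDisparar is true, spawns a BP_Flecha with velocity aimed at TargetArquero's current location.
; Setter functions supply the target and firing permission.
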(event `self.ReceiveBeginPlay`
  (`KismetSystemLibrary.K2_SetTimerDelegate` (delegate `Disparar`) (`self.TiempoDisparo`) true false 0.1))

(event `Disparar`
  (if (`self.PuedeDisparar`)
    (`self.DispararFlechaOrco` (`KismetMathLibrary.Normal` (- (`self.K2_GetActorLocation` (`self.Target Arquero`)) (`self.K2_GetActorLocation`))))))

(event `self.ReceiveTick`
  (params (DeltaSeconds :type "Float (single-precision)"))
  (`self.K2_AddActorLocalOffset` (`self.VectorOrco`)))

(fn `DispararFlechaOrco`
  (params (VelocidadNormalizada :type "Vector Structure"))
  (`|SpawnActorFromClass` "/Game/BP_Flecha.BP_Flecha_C" (`KismetMathLibrary.MakeTransform` (`self.K2_GetActorLocation`)) "Undefined" "OverrideRootScale" null (* VelocidadNormalizada (`self.MultiplicadorVelocidadFlecha`)) null))

(fn `SetPosicionOrco`
  (params (VectorOrco :type "Vector Structure"))
  (set `self.VectorOrco` (* VectorOrco (`self.FactorMultiplicadorVelocidad`))))

(fn `SetPuedeDisparar`
  (params (PuedeDisparar :type Boolean))
  (set `self.PuedeDisparar` PuedeDisparar))

(fn `SetTarget`
  (params (Target :type "Actor Object Reference"))
  (set `self.Target Arquero` Target))

(fn `UserConstructionScript`)